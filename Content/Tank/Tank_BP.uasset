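; Player-controllable tank Blueprint that wires input to movement, aiming and camera components.
; On BeginPlay it passes the barrel and turret to TankAiming and both tracks to TankMovement.
; Drive axes send movement intents to TankMovement, and the Fire action calls TankAiming.
; Aim axes orbit the camera by yawing the azimuth gimbal and pitching the spring arm separately, scaled by delta time.
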(event `self.ReceiveBeginPlay`
  ;[1 1 1] Setting Barrel reference
  (`TankAimingComponent.Initialize` (`self.TankAiming`) (`self.Barrel`) (`self.Turret`))
  (`TankMovementComponent.Initialize` (`self.TankMovement`) (`self.LeftTrack`) (`self.RightTrack`)))

(event `InputAxis|AimAzimuth`
  (params (AxisValue :type "Float (single-precision)"))
  ;[1 1 1] Camera input binding
  (`SceneComponent.K2_AddLocalRotation` (`self.Azimath Gimbal`) (`KismetMathLibrary.MakeRotator` 0.0 0.0 (* AxisValue (`GameplayStatics.GetWorldDeltaSeconds`) 100.0)) false false))

(event `InputAxis|Forward`
  (params (AxisValue :type "Float (single-precision)"))
  ;[1 1 1] Input binding
  (`TankMovementComponent.IntendToMoveForward` (`self.TankMovement`) AxisValue))

(event `InputAxis|Backward`
  (params (AxisValue :type "Float (single-precision)"))
  ;[1 1 1] Input binding
  (`TankMovementComponent.IntendToMoveForward` (`self.TankMovement`) AxisValue))

(event `InputAxis|AimElevation`
  (params (AxisValue :type "Float (single-precision)"))
  ;[1 1 1] Camera input binding
  (`SceneComponent.K2_AddLocalRotation` (`self.SpringArm`) (`KismetMathLibrary.MakeRotator` 0.0 (* AxisValue (`GameplayStatics.GetWorldDeltaSeconds`) 50.0)) false false))

(event `InputAxis|Right`
  (params (AxisValue :type "Float (single-precision)"))
  ;[1 1 1] Input binding
  (`TankMovementComponent.IntendMoveRight` (`self.TankMovement`) AxisValue))

(event `InputAxis|Left`
  (params (AxisValue :type "Float (single-precision)"))
  ;[1 1 1] Input binding
  (`TankMovementComponent.IntendMoveRight` (`self.TankMovement`) AxisValue))

(event `InputAction|Fire`
  (params (Key :type "Key Structure" :default "AnyKey"))
  ;[1 1 1] Camera input binding
  (:`Pressed`
    (`TankAimingComponent.Fire` (`self.TankAiming`))))

(fn `UserConstructionScript`)